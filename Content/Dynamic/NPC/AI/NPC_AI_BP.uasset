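; AI controller for guard NPCs that runs the GuardBehaviour behavior tree on a PatrolData blackboard.
; Perception updates write sensed actors without the "Enemy" tag to the blackboard's enemy key, and clear it when sensing fails.
; Each tick, it sets the controlled TPCharacter's aiming and shooting flags to whether a valid focus actor exists, so the NPC fires whenever it has focus.
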(event OnTargetPerceptionUpdated(AIPerception)
  (params (Actor :type Actor%20Object%20Reference) (Stimulus :type AI%20Stimulus%20Structure))
  (bind _enemykey (Variables|Default|GetEnemyKey))
  (bind _blackboardcomp (Variables|Default|GetBlackboardComp))
  (if (not (Actor|ActorHasTag Actor "Enemy"))
    (if (|BreakAIStimulus Stimulus)
      (AI|Components|Blackboard|SetValueasObject _blackboardcomp _enemykey Actor)
      (else
        (AI|Components|Blackboard|ClearValue _blackboardcomp _enemykey)))))

(event EventBeginPlay
  (bind _blackboardcomponent (Class|AIController|UseBlackboard "/Game/Dynamic/NPC/AI/PatrolData.PatrolData"))
  (AI|RunBehaviorTree "/Game/Dynamic/NPC/AI/GuardBehaviour.GuardBehaviour")
  (Variables|Default|SetBlackboardComp _blackboardcomponent))

(event EventTick
  (params (DeltaSeconds :type Float%20%28single-precision%29))
  (bind _astpcharacter (Utilities|Casting|CastToTPCharacter (Pawn|GetControlledPawn)))
  (bind _output_get (Variables|/Game/Dynamic/NPC/Behaviour/TPCharacter.TPCharacter_C|SetAiming_BP _astpcharacter (Utilities|IsValid (Class|AIController|GetFocusActor))))
  (Variables|/Game/Dynamic/NPC/Behaviour/TPCharacter.TPCharacter_C|SetShooting _astpcharacter _output_get))

(fn ConstructionScript)