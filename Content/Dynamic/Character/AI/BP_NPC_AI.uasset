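; BP_NPC_AI is an AI controller for guard NPCs that runs the BT_GuardBehaviour tree with the BB_PatrolData blackboard.
; Its AIPerception component feeds target updates into a helper that ignores actors tagged "Enemy".
; For any other actor, the helper writes it to EnemyKey when successfully sensed and clears the key when sensing is lost.
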(event OnTargetPerceptionUpdated(AIPerception)
  (params (Actor :type Actor%20Object%20Reference) (Stimulus :type AI%20Stimulus%20Structure))
  (CallFunction|UpdateBlackboardEnemyKey Actor Actor Stimulus))

(event EventBeginPlay
  (bind _blackboardcomponent (Class|AIController|UseBlackboard "/Game/Dynamic/Character/AI/BB_PatrolData.BB_PatrolData"))
  (AI|RunBehaviorTree "/Game/Dynamic/Character/AI/BT_GuardBehaviour.BT_GuardBehaviour")
  (Variables|Default|SetBlackboardComp _blackboardcomponent))

(fn ConstructionScript)

(fn UpdateBlackboardEnemyKey
  (params (ObjectValue :type Object%20Object%20Reference) (self2 :type Actor%20Object%20Reference) (AIStimulus :type AI%20Stimulus%20Structure%20%28by%20ref%29))
  (bind _enemykey (Variables|Default|GetEnemyKey))
  (bind _blackboardcomp (Variables|Default|GetBlackboardComp))
  (if (not (Actor|ActorHasTag self2 "Enemy"))
    (if (.bSuccessfullySensed (Utilities|Struct|BreakAIStimulus AIStimulus))
      (AI|Components|Blackboard|SetValueasObject _blackboardcomp _enemykey ObjectValue)
      (else
        (AI|Components|Blackboard|ClearValue _blackboardcomp _enemykey)))))