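; BP_Tile is a terrain tile for infinite terrain generation that fills itself with random props and gates player movement.
; On BeginPlay it locks its barrier and calls PlaceActors for containers, boxes, canisters, rocks and sacks.
; The player entering LockingVolume turns the barrier green and passable; leaving relocks it red and asks the game mode to spawn another tile.
; GetAttachLocation exposes an arrow transform, and DestroyVolume destroys the tile on player overlap.
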(event OnComponentBeginOverlap(LockingVolume)
  (params (OverlappedComponent :type Primitive%20Component%20Object%20Reference) (OtherActor :type Actor%20Object%20Reference) (OtherComp :type Primitive%20Component%20Object%20Reference) (OtherBodyIndex :type Integer) (bFromSweep :type Boolean) (SweepResult :type Hit%20Result%20Structure%20%28by%20ref%29))
  (Utilities|IsPlayerActor OtherActor)
  (CallFunction|Unlock))

(event OnComponentEndOverlap(LockingVolume)
  (params (OverlappedComponent :type Primitive%20Component%20Object%20Reference) (OtherActor :type Actor%20Object%20Reference) (OtherComp :type Primitive%20Component%20Object%20Reference) (OtherBodyIndex :type Integer))
  (Utilities|IsPlayerActor OtherActor)
  (CallFunction|Lock)
  (bind _asbp_infinite_terrain_game_mode (Utilities|Casting|CastToBP_InfiniteTerrainGameMode (Game|GetGameMode)))
  (Default|SpawnTile _asbp_infinite_terrain_game_mode))

(event OnComponentBeginOverlap(DestroyVolume)
  (params (OverlappedComponent :type Primitive%20Component%20Object%20Reference) (OtherActor :type Actor%20Object%20Reference) (OtherComp :type Primitive%20Component%20Object%20Reference) (OtherBodyIndex :type Integer) (bFromSweep :type Boolean) (SweepResult :type Hit%20Result%20Structure%20%28by%20ref%29))
  (Utilities|IsPlayerActor OtherActor)
  (Actor|DestroyActor))

(event EventBeginPlay
  (CallFunction|Lock)
  (Class|TileCPP|PlaceActors "/Game/Dynamic/Terrain/Props/BP_Container.BP_Container_C" 1 3)
  (Class|TileCPP|PlaceActors "/Game/Dynamic/Terrain/Props/BP_Box.BP_Box_C" 2 4)
  (Class|TileCPP|PlaceActors "/Game/Dynamic/Terrain/Props/BP_Canister.BP_Canister_C" 3 7)
  (Class|TileCPP|PlaceActors "/Game/Dynamic/Terrain/Props/BP_Rock.BP_Rock_C" 0 4)
  (Class|TileCPP|PlaceActors "/Game/Dynamic/Terrain/Props/BP_Rock02.BP_Rock02_C" 0 4)
  (Class|TileCPP|PlaceActors "/Game/Dynamic/Terrain/Props/BP_Rock03.BP_Rock03_C" 0 4)
  (Class|TileCPP|PlaceActors "/Game/Dynamic/Terrain/Props/BP_Sack.BP_Sack_C" 1 2))

(event Collision|EventActorBeginOverlap
  (params (OtherActor :type Actor%20Object%20Reference)))

(event EventTick
  (params (DeltaSeconds :type Float%20%28single-precision%29)))

(fn ConstructionScript)

(fn GetAttachLocation
  (return (Transformation|GetWorldTransform (Variables|Default|GetArrow))))

(fn Unlock
  (bind _barrier (Variables|Default|GetBarrier))
  (Collision|SetCollisionEnabled _barrier "NoCollision")
  (Rendering|Material|SetMaterial _barrier 0 "/Game/Dynamic/Terrain/MI_Barrier_Green.MI_Barrier_Green"))

(fn Lock
  (bind _barrier (Variables|Default|GetBarrier))
  (Collision|SetCollisionEnabled _barrier "QueryAndPhysics")
  (Rendering|Material|SetMaterial _barrier 0 "/Game/Dynamic/Terrain/MI_Barrier_Red.MI_Barrier_Red"))